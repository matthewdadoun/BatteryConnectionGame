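; Backup Blueprint holding what looks like level audio logic for fading sounds in and out around the first-person character, with nothing wired to run.
; Orphaned chains cast to BP_FirstPersonCharacter, then either unpause and fade in an audio component, or fade it out and pause it after a matching delay.
; Another orphaned node pauses three audio components at once, and the construction script is empty.
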(fn ConstructionScript)