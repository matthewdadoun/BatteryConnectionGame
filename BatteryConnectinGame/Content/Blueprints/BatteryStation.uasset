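; Battery station Blueprint that plays the visual and audio feedback when a battery is placed in or removed from it.
; PlayBatteryAnimation shows or hides the battery mesh by the placed flag, then after a delay toggles the indicator inversely and plays a placement sound.
; When placed, it also spins the battery, then plays a charge-up sound and swaps a station material to its charged look.
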(event EventPlayBatteryAnimation
  (params (bBatteryPlaced :type Boolean))
  (Rendering|SetVisibility (Variables|Default|Getbattery) bBatteryPlaced false)
  (Utilities|FlowControl|Delay 2.0)
  (Rendering|SetVisibility (Variables|Default|Getindicator) (not bBatteryPlaced) false)
  (Audio|Components|Audio|Play (Variables|Default|GetBatteryPlaced) 0.0)
  (Utilities|FlowControl|Delay 0.3)
  (if bBatteryPlaced
    (Components|Animation|PlayAnimation (Variables|Default|Getbattery) "/Game/Models/batteryStuff/battery_Anim_batterySkel_Spin.battery_Anim_batterySkel_Spin" false)
    (Utilities|FlowControl|Delay 1.3)
    (Audio|Components|Audio|Play (Variables|Default|GetChargeUp) 0.0)
    (Rendering|Material|SetMaterial (Variables|Default|Getstation) 1 "/Game/Models/batteryStuff/charge.charge")))

(fn ConstructionScript)